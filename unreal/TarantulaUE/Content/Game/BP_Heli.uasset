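; Rescue helicopter that circles on an elliptical patrol until Rescue hands it a target to pick up.
; A Tick state machine flies it over the target, descends, waits briefly, marks the target boarded and hidden, then climbs away and hides.
; FlyTo steers every leg with smoothed yaw and speed-based pitch.
; Setup assembles component parts and sets red or blue variant orbits, while Tick animates rotors, beacon and camera-distance rotor volume.
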(event `self.ReceiveBeginPlay`
  (`self.Setup`))

(event `self.ReceiveTick`
  (params (DeltaSeconds :type "Float (single-precision)"))
  (bind _returnvalue (`self.K2_GetActorLocation`))
  (bind _returnvalue_2 (`KismetMathLibrary.FMin` DeltaSeconds 0.05))
  (bind _returnvalue_3 (`self.K2_GetActorLocation` (`self.Target`)))
  (set `self.T` (+ (`self.T`) _returnvalue_2))
  (bind _v (`self.CamVol` (`self.K2_GetActorLocation`) 16000.0))
  (set `AudioComponent.VolumeMultiplier` (* 0.8 _v) (`self.Rotor`))
  (`SceneComponent.K2_AddLocalRotation` (`self.Hub`) (`KismetMathLibrary.MakeRotator` 0.0 0.0 (* 1300.0 _returnvalue_2)) false false)
  (`SceneComponent.K2_AddLocalRotation` (`self.TailHub`) (`KismetMathLibrary.MakeRotator` 0.0 (* 2000.0 _returnvalue_2)) false false)
  (`LightComponent.SetIntensity` (`self.Beacon`) (select `bool` (< (mod (`self.T`) 1.0) 0.12) :`false` 0.0 :`true` 60000.0))
  (if (== (`self.Mode`) 0)
    (set `self.Ang` (+ (`self.Ang`) (* (* (`self.Dir`) 0.11) _returnvalue_2)))
    (`self.FlyTo` (`KismetMathLibrary.MakeVector` (* (`self.RX`) (`KismetMathLibrary.Cos` (`self.Ang`))) (* (`self.RY`) (`KismetMathLibrary.Sin` (`self.Ang`))) (+ (`self.Alt`) (* 120.0 (`KismetMathLibrary.Sin` (* (`self.T`) 0.5))))) 700.0 _returnvalue_2))
  (bind _ok (`self.Valid` (`self.Target`)))
  (if (and (== (`self.Mode`) 1) _ok)
    (bind _arrived (`self.FlyTo` (`KismetMathLibrary.MakeVector` (.x _returnvalue_3) (.y _returnvalue_3) (`self.Alt`)) 1100.0 _returnvalue_2))
    (if _arrived
      (set `self.Mode` 2)))
  (if (and (== (`self.Mode`) 2) _ok)
    (bind _arrived_2 (`self.FlyTo` (+ (`self.K2_GetActorLocation` (`self.Target`)) (`KismetMathLibrary.MakeVector` 0.0 0.0 480.0)) 380.0 _returnvalue_2))
    (if _arrived_2
      (set `self.Mode` 3)
      (set `self.T` 0.0)))
  (if (and (== (`self.Mode`) 3) (> (`self.T`) 2.5))
    (if _ok
      (set `/Game/Game/BP_Human.Boarded` true (`self.Target`))
      (`self.SetActorHiddenInGame` (`self.Target`) true))
    (set `self.Mode` 4))
  (if (== (`self.Mode`) 4)
    (bind _arrived_3 (`self.FlyTo` (`KismetMathLibrary.MakeVector` (.x _returnvalue) (.y _returnvalue) 8000.0) 700.0 _returnvalue_2))
    (if _arrived_3
      (set `self.Done` true)
      (`self.SetActorHiddenInGame` self true)))
  (if (and (and (>= (`self.Mode`) 1) (<= (`self.Mode`) 2)) (not _ok))
    (set `self.Mode` 4)))

(fn `CamVol`
  (params (P :type "Vector Structure") (Far :type "Float (double-precision)"))
  (returns (V :type "Float (double-precision)"))
  (return (`KismetMathLibrary.FClamp` (- 1.0 (/ (`KismetMathLibrary.Vector_Distance` (`PlayerCameraManager.GetCameraLocation` (`GameplayStatics.GetPlayerCameraManager` 0)) P) Far)))))

(fn `FlyTo`
  (params (P :type "Vector Structure") (Spd :type "Float (double-precision)") (DT :type "Float (double-precision)"))
  (returns (Arrived :type Boolean))
  (bind _returnvalue (`self.K2_GetActorLocation`))
  (bind _returnvalue_2 (- P _returnvalue))
  (bind _returnvalue_3 (`KismetMathLibrary.VSize` _returnvalue_2))
  (if (> (`KismetMathLibrary.VSize` (`KismetMathLibrary.MakeVector` (.x _returnvalue_2) (.y _returnvalue_2))) 50.0)
    (set `self.Yaw` (`KismetMathLibrary.FInterpTo` (`self.Yaw`) (+ (`self.Yaw`) (`KismetMathLibrary.NormalizeAxis` (- (`KismetMathLibrary.DegAtan2` (.y _returnvalue_2) (.x _returnvalue_2)) (`self.Yaw`)))) DT 1.5)))
  (`self.K2_SetActorLocationAndRotation` self (+ _returnvalue (* (`KismetMathLibrary.Normal` _returnvalue_2) (`KismetMathLibrary.FMin` _returnvalue_3 (* Spd DT)))) (`KismetMathLibrary.MakeRotator` 0.0 (`KismetMathLibrary.FClamp` (/ (* Spd -0.01) 1.0) -10.0 0.0) (`self.Yaw`)) false false)
  (return (< _returnvalue_3 60.0)))

(fn `Part`
  (params (C :type "SceneComponent Object Reference") (L :type "Vector Structure") (R :type "Rotator Structure") (S :type "Vector Structure"))
  (`SceneComponent.K2_SetRelativeTransform` C (`KismetMathLibrary.MakeTransform` L R S) false false))

(fn `Rescue`
  (params (Who :type "/Game/Game/BP_Human Object Reference"))
  (set `self.Target` Who)
  (set `self.Busy` true)
  (set `self.Mode` 1))

(fn `Setup`
  (bind _returnvalue (`KismetMathLibrary.MakeRotator` 0.0))
  (bind _returnvalue_2 (`KismetMathLibrary.MakeRotator` 0.0 90.0))
  (bind _returnvalue_3 (== (`self.Color`) 0))
  (for _array_element (`self.K2_GetComponentsByClass` self "/Script/Engine.PrimitiveComponent")
    (`PrimitiveComponent.SetCollisionEnabled` _array_element "NoCollision"))
  (`self.Part` (`self.Body`) (`KismetMathLibrary.MakeVector` 0.0) _returnvalue (`KismetMathLibrary.MakeVector` 6.0 2.6 2.5))
  (`self.Part` (`self.Glass`) (`KismetMathLibrary.MakeVector` 180.0 0.0 30.0) _returnvalue (`KismetMathLibrary.MakeVector` 2.8 2.2 1.8))
  (`self.Part` (`self.Tail`) (`KismetMathLibrary.MakeVector` -620.0 0.0 50.0) _returnvalue_2 (`KismetMathLibrary.MakeVector` 0.45 0.45 6.5))
  (`self.Part` (`self.Fin`) (`KismetMathLibrary.MakeVector` -940.0 0.0 150.0) _returnvalue (`KismetMathLibrary.MakeVector` 0.9 0.1 1.8))
  (`self.Part` (`self.SkidL`) (`KismetMathLibrary.MakeVector` 0.0 -120.0 -170.0) _returnvalue_2 (`KismetMathLibrary.MakeVector` 0.12 0.12 5.0))
  (`self.Part` (`self.SkidR`) (`KismetMathLibrary.MakeVector` 0.0 120.0 -170.0) _returnvalue_2 (`KismetMathLibrary.MakeVector` 0.12 0.12 5.0))
  (`self.Part` (`self.Hub`) (`KismetMathLibrary.MakeVector` 0.0 0.0 150.0) _returnvalue (`KismetMathLibrary.MakeVector` 1.0 1.0 1.0))
  (`self.Part` (`self.Blade1`) (`KismetMathLibrary.MakeVector` 0.0) _returnvalue (`KismetMathLibrary.MakeVector` 12.0 0.35 0.06))
  (`self.Part` (`self.Blade2`) (`KismetMathLibrary.MakeVector` 0.0) _returnvalue (`KismetMathLibrary.MakeVector` 0.35 12.0 0.06))
  (`self.Part` (`self.TailHub`) (`KismetMathLibrary.MakeVector` -950.0 25.0 150.0) _returnvalue (`KismetMathLibrary.MakeVector` 1.0 1.0 1.0))
  (`self.Part` (`self.TBlade`) (`KismetMathLibrary.MakeVector` 0.0) _returnvalue (`KismetMathLibrary.MakeVector` 2.2 0.05 0.25))
  (`self.Part` (`self.Search`) (`KismetMathLibrary.MakeVector` 250.0 0.0 -180.0) (`KismetMathLibrary.MakeRotator` 0.0 -70.0) (`KismetMathLibrary.MakeVector` 1.0 1.0 1.0))
  (`self.Part` (`self.Beacon`) (`KismetMathLibrary.MakeVector` 0.0 0.0 -260.0) _returnvalue (`KismetMathLibrary.MakeVector` 1.0 1.0 1.0))
  (if _returnvalue_3
    (`PrimitiveComponent.SetMaterial` (`self.Body`) 0 "/Game/Game/Mat/MI_HeliRed.MI_HeliRed")
    (`PrimitiveComponent.SetMaterial` (`self.Tail`) 0 "/Game/Game/Mat/MI_HeliRed.MI_HeliRed")
    (`PrimitiveComponent.SetMaterial` (`self.Fin`) 0 "/Game/Game/Mat/MI_HeliRed.MI_HeliRed")
    (else
      (`PrimitiveComponent.SetMaterial` (`self.Body`) 0 "/Game/Game/Mat/MI_HeliBlue.MI_HeliBlue")
      (`PrimitiveComponent.SetMaterial` (`self.Tail`) 0 "/Game/Game/Mat/MI_HeliBlue.MI_HeliBlue")
      (`PrimitiveComponent.SetMaterial` (`self.Fin`) 0 "/Game/Game/Mat/MI_HeliBlue.MI_HeliBlue")))
  (`PrimitiveComponent.SetMaterial` (`self.Glass`) 0 "/Game/Game/Mat/MI_Glass.MI_Glass")
  (`PrimitiveComponent.SetMaterial` (`self.SkidL`) 0 "/Game/Game/Mat/MI_Black.MI_Black")
  (`PrimitiveComponent.SetMaterial` (`self.SkidR`) 0 "/Game/Game/Mat/MI_Black.MI_Black")
  (`PrimitiveComponent.SetMaterial` (`self.Blade1`) 0 "/Game/Game/Mat/MI_Black.MI_Black")
  (`PrimitiveComponent.SetMaterial` (`self.Blade2`) 0 "/Game/Game/Mat/MI_Black.MI_Black")
  (`PrimitiveComponent.SetMaterial` (`self.TBlade`) 0 "/Game/Game/Mat/MI_Black.MI_Black")
  (`LightComponent.SetLightColor` (`self.Beacon`) (select `bool` _returnvalue_3 :`false` (`KismetMathLibrary.MakeColor` 0.2 0.4 1.0 1.0) :`true` (`KismetMathLibrary.MakeColor` 1.0 0.1 0.05 1.0)) true)
  (set `self.Alt` (select `bool` _returnvalue_3 :`false` 3300.0 :`true` 4300.0))
  (set `self.RX` (select `bool` _returnvalue_3 :`false` 3800.0 :`true` 4600.0))
  (set `self.RY` (select `bool` _returnvalue_3 :`false` 2200.0 :`true` 2700.0))
  (set `self.Dir` (select `bool` _returnvalue_3 :`false` -1.0 :`true` 1.0))
  (set `self.Ang` (select `bool` _returnvalue_3 :`false` 3.1 :`true` 0.0)))

(fn `UserConstructionScript`)

(fn `Valid`
  (params (A :type "Actor Object Reference"))
  (returns (Ok :type Boolean))
  (`/Engine/EditorBlueprintResources/StandardMacros.IsValid` A
    (:`Is Valid`
      (return true))
    (:`Is Not Valid`
      (return false))))