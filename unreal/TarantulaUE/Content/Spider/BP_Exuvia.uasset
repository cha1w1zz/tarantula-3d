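; BP_Exuvia is the shed skin of a spider, a static, collision-free, pale replica of a spider's current pose.
; Copy clones the source spider's body and abdomen meshes plus its instanced leg and knob transforms, setting a "Pale" material parameter.
; It drops slightly on creation, and after three minutes Tick sinks it at a speed scaled by the spider's Span, then destroys it ten seconds later.
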(event `self.ReceiveTick`
  (params (DeltaSeconds :type "Float (single-precision)"))
  (set `self.Life` (+ (`self.Life`) DeltaSeconds))
  (if (> (`self.Life`) 180.0)
    (`self.K2_AddActorWorldOffset` self (`KismetMathLibrary.MakeVector` 0.0 0.0 (* (* DeltaSeconds (`self.Sink`)) -1.0)) false false)
    (if (> (`self.Life`) 190.0)
      (`self.K2_DestroyActor` self))))

(fn `Copy`
  (params (S :type "/Game/Spider/BP_Tarantula Object Reference"))
  (bind _span (`/Game/Spider/BP_Tarantula.Span` S))
  (`self.CopyMesh` (`/Game/Spider/BP_Tarantula.Body` S) (`self.Body`))
  (`self.CopyMesh` (`/Game/Spider/BP_Tarantula.Abdomen` S) (`self.Abdomen`))
  (`self.CopyISM` (`/Game/Spider/BP_Tarantula.Legs` S) (`self.Legs`) 8)
  (`self.CopyISM` (`/Game/Spider/BP_Tarantula.LegB` S) (`self.LegB`) 8)
  (`self.CopyISM` (`/Game/Spider/BP_Tarantula.LegC` S) (`self.LegC`) 8)
  (`self.CopyISM` (`/Game/Spider/BP_Tarantula.LegT` S) (`self.LegT`) 8)
  (`self.CopyISM` (`/Game/Spider/BP_Tarantula.Knobs` S) (`self.Knobs`) 24)
  (set `self.Sink` (* _span 0.012))
  (`self.K2_AddActorWorldOffset` self (`KismetMathLibrary.MakeVector` 0.0 0.0 (* _span -0.025)) false false))

(fn `CopyISM`
  (params (From :type "InstancedStaticMeshComponent Object Reference") (To :type "InstancedStaticMeshComponent Object Reference") (N :type Integer))
  (`StaticMeshComponent.SetStaticMesh` To (`StaticMeshComponent.StaticMesh` From))
  (`InstancedStaticMeshComponent.ClearInstances` To)
  (`PrimitiveComponent.SetCollisionEnabled` To "NoCollision")
  (for _index (range (+ (- N 1) 1))
    (`InstancedStaticMeshComponent.AddInstance` To (`InstancedStaticMeshComponent.GetInstanceTransform` From _index true) true))
  (`MeshComponent.SetScalarParameterValueOnMaterials` To "Pale" 1.0))

(fn `CopyMesh`
  (params (From :type "StaticMeshComponent Object Reference") (To :type "StaticMeshComponent Object Reference"))
  (`StaticMeshComponent.SetStaticMesh` To (`StaticMeshComponent.StaticMesh` From))
  (`SceneComponent.K2_SetWorldTransform` To (`SceneComponent.K2_GetComponentToWorld` From) false false)
  (`PrimitiveComponent.SetCollisionEnabled` To "NoCollision")
  (`MeshComponent.SetScalarParameterValueOnMaterials` To "Pale" 1.0))

(fn `UserConstructionScript`)